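; Player controller for the GB game that sets up the local player's UI.
; On InitializePlayerUI, it creates WBP_PrimaryLayout, adds it to the viewport and registers it with GBUISubsystem.
; It then passes the Ability System Component to the subsystem's HUD setup and makes the HUD visible.
; BeginPlay and Tick are empty, and an Enhanced Input registration of IMC_Gameplay is left unconnected, so it never runs.
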(event EventBeginPlay)

(event EventTick
  (params (DeltaSeconds :type Float%20%28single-precision%29)))

(event EventInitializePlayerUI
  (bind _returnvalue (Subsystems|GetGBUISubsystem))
  (Utilities|FlowControl|Sequence
    (:then_0
      (bind _returnvalue_2 (UserInterface|CreateWidget "/Game/GB/UI/InGame/Widgets/WBP_PrimaryLayout.WBP_PrimaryLayout_C" self))
      (UserInterface|Viewport|AddtoViewport _returnvalue_2 0)
      (Class|GBUISubsystem|RegisterCreatedPrimaryLayoutWidget (Subsystems|GetGBUISubsystem) _returnvalue_2)
      (bind _returnvalue_3 (Class|GBPlayerController|GetAbilitySystemComponent))
      (Class|GBUISubsystem|SetHUDWidget _returnvalue _returnvalue_3)
      (Class|GBUISubsystem|SetHUDVisible _returnvalue true))))

(fn ConstructionScript)