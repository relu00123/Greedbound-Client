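; Stun field actor that repeatedly applies the SturnGE gameplay effect to characters standing inside its box.
; A looping one-second timer started on BeginPlay runs on authority only and gathers GBCharacterBase actors overlapping the Box.
; Each actor with a valid Ability System Component applies the effect spec to itself, with the Data.Damage.Impact SetByCaller magnitude set to zero.
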(event Custom|커스텀이벤트
  (Networking|SwitchHasAuthority
    (:Authority
      (for _array_element (Collision|GetOverlappingActors (Variables|Default|GetBox) "/Script/Greedbound.GBCharacterBase" :!class /Script/Engine.PrimitiveComponent)
        (if (Utilities|IsValid (Ability|GetAbilitySystemComponent _array_element))
          (bind _returnvalue (Ability|GameplayEffect|AssignTagSetbyCallerMagnitude (GameplayEffects|MakeOutgoingSpec (Ability|GetAbilitySystemComponent _array_element) (Variables|Default|GetSturnGE) 0.0 (GameplayEffects|MakeEffectContext (Ability|GetAbilitySystemComponent _array_element))) "(TagName=\"Data.Damage.Impact\")" 0.0))
          (GameplayEffects|ApplyGameplayEffectSpecToSelf (Ability|GetAbilitySystemComponent _array_element) _returnvalue))))))

(event EventBeginPlay
  (Utilities|Time|SetTimerbyEvent (delegate Custom|커스텀이벤트) 1.0 true true))

(event Collision|EventActorBeginOverlap
  (params (OtherActor :type Actor%20Object%20Reference)))

(event EventTick
  (params (DeltaSeconds :type Float%20%28single-precision%29)))

(fn ConstructionScript)