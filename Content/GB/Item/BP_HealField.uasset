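; BP_HealField is an area actor that periodically heals characters standing inside its box.
; A looping timer, started on BeginPlay, polls GBCharacterBase overlaps on the authority.
; Each target's ability system applies two Gameplay Effects to itself: a heal-over-time with set duration and an impact heal.
; Amounts are passed through SetByCaller using Data.Damage tags, and both effects are reapplied every tick of the timer.
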(event Custom|커스텀이벤트
  (Networking|SwitchHasAuthority
    (:Authority
      (for _array_element (Collision|GetOverlappingActors (Variables|Default|GetBox) "/Script/Greedbound.GBCharacterBase" :!class /Script/Engine.PrimitiveComponent)
        (if (Utilities|IsValid (Ability|GetAbilitySystemComponent _array_element))
          (bind _returnvalue (Ability|GameplayEffect|AssignTagSetbyCallerMagnitude (GameplayEffects|MakeOutgoingSpec (Ability|GetAbilitySystemComponent _array_element) (Variables|Default|GetDotGE) 0.0 (GameplayEffects|MakeEffectContext (Ability|GetAbilitySystemComponent _array_element))) "(TagName=\"Data.Damage.Dot\")" (Variables|Default|GetDotHeal)))
          (bind _returnvalue_2 (Ability|GameplayEffect|AssignTagSetbyCallerMagnitude _returnvalue "(TagName=\"Data.Damage.DotDuration\")" (Variables|Default|GetDotDuration)))
          (GameplayEffects|ApplyGameplayEffectSpecToSelf (Ability|GetAbilitySystemComponent _array_element) _returnvalue_2)
          (bind _returnvalue_3 (Ability|GameplayEffect|AssignTagSetbyCallerMagnitude (GameplayEffects|MakeOutgoingSpec (Ability|GetAbilitySystemComponent _array_element) (Variables|Default|GetImpactGE) 0.0 (GameplayEffects|MakeEffectContext (Ability|GetAbilitySystemComponent _array_element))) "(TagName=\"Data.Damage.Impact\")" (Variables|Default|GetImpactHeal)))
          (GameplayEffects|ApplyGameplayEffectSpecToSelf (Ability|GetAbilitySystemComponent _array_element) _returnvalue_3))))))

(event EventBeginPlay
  (Utilities|Time|SetTimerbyEvent (delegate Custom|커스텀이벤트) (Variables|Default|GetOverlapFrequency) true true))

(event Collision|EventActorBeginOverlap
  (params (OtherActor :type Actor%20Object%20Reference)))

(event EventTick
  (params (DeltaSeconds :type Float%20%28single-precision%29)))

(fn ConstructionScript)